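; BP_PhysicsVehicle is a possessable physics vehicle that rides on raycast suspension, with no drive or steering logic yet.
; Each tick, all four wheel points trace downward along their local up axis to the suspension rest distance.
; On a hit, a damped spring force, scaled by delta time, pushes the Box body at that wheel, with debug trace and arrow drawing.
; Possession adds an Enhanced Input mapping context.
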(event `self.ReceivePossessed`
  (params (NewController :type "Controller Object Reference"))
  (bind _asbp_player_controller (cast `/Game/Bluepirnts/BP_PlayerController` NewController))
  (bind _output_get (set `self.As BP Player Controller` _asbp_player_controller))
  (`EnhancedInputSubsystemInterface.AddMappingContext` (pcsubsystem `EnhancedInputLocalPlayerSubsystem` _output_get) null 0 (struct)))

(event `self.ReceiveTick`
  (params (DeltaSeconds :type "Float (single-precision)"))
  (`self.HandleWheelForces` (`self.FL_Wheel`))
  (`self.HandleWheelForces` (`self.FR_Wheel`))
  (`self.HandleWheelForces` (`self.BR_Wheel`))
  (`self.HandleWheelForces` (`self.BL_Wheel`)))

(fn `CalculateSuspension`
  (params (CurrentWheel :type "SceneComponent Object Reference") (OutDist :type "Float (double-precision)"))
  (bind _returnvalue (`SceneComponent.K2_GetComponentLocation` (`local.CurrentWheel`)))
  (bind _returnvalue_2 (`PrimitiveComponent.GetPhysicsLinearVelocityAtPoint` (`self.Box`) (`SceneComponent.K2_GetComponentLocation` (`local.CurrentWheel`)) "None"))
  (bind _returnvalue_3 (* (`SceneComponent.GetUpVector` (`local.CurrentWheel`)) (- (* (- (`self.SuspensionRestDist`) OutDist) (`self.SpringForce`)) (* (`self.SpringDamper`) (`KismetMathLibrary.Dot_VectorVector` _returnvalue_2 (`SceneComponent.GetUpVector` CurrentWheel)))) (`GameplayStatics.GetWorldDeltaSeconds`)))
  (`PrimitiveComponent.AddForceAtLocation` (`self.Box`) _returnvalue_3 _returnvalue "None")
  (`KismetSystemLibrary.DrawDebugArrow` _returnvalue (+ (* _returnvalue_3 0.0005) _returnvalue) 0.0 (struct :`R` 0.187065 :`G` 1.0 :`A` 1.0)))

(fn `HandleWheelForces`
  (params (`Current Wheel` :type "SceneComponent Object Reference"))
  (bind _returnvalue (`SceneComponent.K2_GetComponentLocation` `Current Wheel`))
  (bind _outhit (`KismetSystemLibrary.LineTraceSingle` :`Start` _returnvalue :`End` (+ (* (`SceneComponent.GetUpVector` `Current Wheel`) -1.0 (`self.SuspensionRestDist`)) _returnvalue) :`TraceChannel` "TraceTypeQuery1" :`DrawDebugType` "ForOneFrame"))
  (if (`GameplayStatics.BreakHitResult` _outhit)
    (`self.CalculateSuspension` (`local.Current Wheel`) (`.Distance` (`GameplayStatics.BreakHitResult` _outhit)))))

(fn `UserConstructionScript`)